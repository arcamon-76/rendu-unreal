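; Player character with two movement modes: Classique for walking and jumping, Liane for climbing vines.
; Enhanced Input handlers switch on the GameMode variable, so move input either walks relative to camera yaw or slides and spins the capsule on the vine.
; SetVariable stores a vine and enables grabbing, which snaps to it and disables gravity.
; Jumping off restores gravity and applies a forward-upward impulse; VerifyPosToRope repositions out-of-range players.
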(event `JumpOutVine`
  (bind (_returnvalue_x _returnvalue_y) (`KismetMathLibrary.BreakVector` (`SceneComponent.GetForwardVector` (`self.CapsuleComponent`))))
  ;[1 1 1] Comment
  (`self.EndVine`)
  (`CharacterMovementComponent.AddImpulse` (`self.CharacterMovement`) (* (`KismetMathLibrary.MakeVector` _returnvalue_x _returnvalue_y 0.5) 75000.0) false))

(event `self.ReceiveBeginPlay`
  ;[1 1 1] Initial
  (bind _asplayer_controller (cast `PlayerController` (`self.GetController`)))
  (bind _returnvalue (pcsubsystem `EnhancedInputLocalPlayerSubsystem` _asplayer_controller))
  (`/Engine/EditorBlueprintResources/StandardMacros.IsValid` _returnvalue
    (:`Is Valid`
      (`EnhancedInputSubsystemInterface.AddMappingContext` _returnvalue "/Game/BluePrint/Character/Player/Input/Actions/IMC_Player.IMC_Player" 0 (struct)))))

(event `EnhancedInput|/Game/BluePrint/Character/Player/Input/Actions/IA_MyLook`
  (params (ActionValue :type "Vector2D Structure") (ElapsedSeconds :type "Float (double-precision)") (TriggeredSeconds :type "Float (double-precision)") (InputAction :type "InputAction Object Reference" :default "/Game/BluePrint/Character/Player/Input/Actions/IA_MyLook.IA_MyLook"))
  ;[1 1 1] PlayerLook
  (:`Triggered`
    (`self.AddControllerYawInput` ActionValue_X)
    (`self.AddControllerPitchInput` ActionValue_Y)))

(event `EnhancedInput|/Game/BluePrint/Character/Player/Input/Actions/IA_MyJump`
  (params (ActionValue :type Boolean) (ElapsedSeconds :type "Float (double-precision)") (TriggeredSeconds :type "Float (double-precision)") (InputAction :type "InputAction Object Reference" :default "/Game/BluePrint/Character/Player/Input/Actions/IA_MyJump.IA_MyJump"))
  ;[1 1 1] PlayerJump
  (:`Started`
    (switch `/Game/BluePrint/Character/Player/GameMode` (`self.GameMode`)
      (:`NewEnumerator0`
        (`self.Jump`))
      (:`NewEnumerator1`
        (`self.JumpOutVine`))))
  (:`Completed`
    (switch `/Game/BluePrint/Character/Player/GameMode` (`self.GameMode`)
      (:`NewEnumerator0`
        (`self.StopJumping`)))))

(event `EnhancedInput|/Game/BluePrint/Character/Player/Input/Actions/IA_MyMove`
  (params (ActionValue :type "Vector2D Structure") (ElapsedSeconds :type "Float (double-precision)") (TriggeredSeconds :type "Float (double-precision)") (InputAction :type "InputAction Object Reference" :default "/Game/BluePrint/Character/Player/Input/Actions/IA_MyMove.IA_MyMove"))
  (bind (_returnvalue_roll _returnvalue_pitch _returnvalue_yaw) (`KismetMathLibrary.BreakRotator` (`self.GetControlRotation`)))
  (bind (_returnvalue_x _returnvalue_y _returnvalue_z) (`KismetMathLibrary.BreakVector` (`self.K2_GetActorLocation`)))
  (bind (_returnvalue_roll_2 _returnvalue_pitch_2 _returnvalue_yaw_2) (`KismetMathLibrary.BreakRotator` (`self.GetControlRotation`)))
  ;[1 1 1] Player Movement
  (:`Triggered`
    (switch `/Game/BluePrint/Character/Player/GameMode` (`self.GameMode`)
      (:`NewEnumerator0`
        (`self.AddMovementInput` (`KismetMathLibrary.GetRightVector` (`KismetMathLibrary.MakeRotator` 0.0 0.0 _returnvalue_yaw)) ActionValue_X)
        (`self.AddMovementInput` (`KismetMathLibrary.GetForwardVector` (`KismetMathLibrary.MakeRotator` 0.0 0.0 _returnvalue_yaw_2)) ActionValue_Y))
      (:`NewEnumerator1`
        (if (> (`KismetMathLibrary.Abs` ActionValue_Y) 0.5)
          (if (> ActionValue_Y 0.0)
            (set `self.VineSpeed` 10.0)
            (else
              (set `self.VineSpeed` -10.0)))
          (`self.K2_SetActorLocation` (`KismetMathLibrary.MakeVector` _returnvalue_x _returnvalue_y (+ _returnvalue_z (`self.VineSpeed`))))
          (else
            (if (> ActionValue_X 0.0)
              (set `self.VineSpeedRotation` 7.5)
              (else
                (set `self.VineSpeedRotation` -7.5)))
            (`SceneComponent.K2_AddLocalRotation` (`self.CapsuleComponent`) (`KismetMathLibrary.MakeRotator` 0.0 0.0 (`self.VineSpeedRotation`)) false false)))))))

(event `EnhancedInput|/Game/BluePrint/Character/Player/Input/Actions/IA_GrabVine`
  (params (ActionValue :type Boolean) (ElapsedSeconds :type "Float (double-precision)") (TriggeredSeconds :type "Float (double-precision)") (InputAction :type "InputAction Object Reference" :default "/Game/BluePrint/Character/Player/Input/Actions/IA_GrabVine.IA_GrabVine"))
  ;[1 1 1] GrabVine
  (:`Started`
    (if (== true (`self.CanGrab`))
      (set `self.CanGrab` false)
      (`self.DoGrab`))))

(event `VerifyPosToRope`
  (bind (_returnvalue_x _returnvalue_y _returnvalue_z) (`KismetMathLibrary.BreakVector` (`self.GetActorScale3D`)))
  (bind (_returnvalue_x_2 _returnvalue_y_2 _returnvalue_z_2) (`KismetMathLibrary.BreakVector` (`self.GetActorScale3D`)))
  (bind _vine (`self.Vine`))
  (bind (_returnvalue_x_3 _returnvalue_y_3 _returnvalue_z_3) (`KismetMathLibrary.BreakVector` (`self.GetActorScale3D` _vine)))
  (bind _rootcomponent (`Actor.RootComponent` (`self.Vine`)))
  (bind _rootcomponent_2 (`Actor.RootComponent` (`self.Vine`)))
  (bind (_returnvalue_x_4 _returnvalue_y_4) (`KismetMathLibrary.BreakVector` (`SceneComponent.K2_GetComponentLocation` _rootcomponent_2)))
  (bind (_returnvalue_x_5 _returnvalue_y_5 _returnvalue_z_4) (`KismetMathLibrary.BreakVector` (`SceneComponent.K2_GetComponentLocation` (`Actor.RootComponent` (`self.Player`)))))
  (bind (_returnvalue_x_6 _returnvalue_y_6 _returnvalue_z_5) (`KismetMathLibrary.BreakVector` (`SceneComponent.K2_GetComponentLocation` _rootcomponent_2)))
  (bind (_returnvalue_x_7 _returnvalue_y_7 _returnvalue_z_6) (`KismetMathLibrary.BreakVector` (`SceneComponent.K2_GetComponentLocation` (`Actor.RootComponent` (`self.Vine`)))))
  (bind (_returnvalue_x_8 _returnvalue_y_8 _returnvalue_z_7) (`KismetMathLibrary.BreakVector` (`SceneComponent.K2_GetComponentLocation` (`Actor.RootComponent` _vine))))
  (bind (_returnvalue_x_9 _returnvalue_y_9 _returnvalue_z_8) (`KismetMathLibrary.BreakVector` (`SceneComponent.K2_GetComponentLocation` (`Actor.RootComponent` (`self.Player`)))))
  (bind (_returnvalue_x_10 _returnvalue_y_10) (`KismetMathLibrary.BreakVector` (`SceneComponent.K2_GetComponentLocation` _rootcomponent)))
  (bind (_returnvalue_x_11 _returnvalue_y_11 _returnvalue_z_9) (`KismetMathLibrary.BreakVector` (`SceneComponent.K2_GetComponentLocation` _rootcomponent)))
  ;[1 1 1] VerifyPosRope
  (if (<= _returnvalue_z_8 (- _returnvalue_z_7 _returnvalue_z_3))
    (`SceneComponent.K2_SetWorldLocation` (`Actor.RootComponent` (`self.Player`)) (`KismetMathLibrary.MakeVector` _returnvalue_x_10 _returnvalue_y_10 (- _returnvalue_z_9 _returnvalue_z_2)) false false)
    (elif (>= _returnvalue_z_4 _returnvalue_z_6)
      (`SceneComponent.K2_SetWorldLocation` (`Actor.RootComponent` (`self.Player`)) (`KismetMathLibrary.MakeVector` _returnvalue_x_4 _returnvalue_y_4 (- _returnvalue_z_5 _returnvalue_z)) false false))))

(event `DoGrab`
  (bind _charactermovement (`self.CharacterMovement`))
  (bind (_vinepos_x _vinepos_y) (`KismetMathLibrary.BreakVector` (`self.VinePos`)))
  (bind (_returnvalue_x _returnvalue_y _returnvalue_z) (`KismetMathLibrary.BreakVector` (`SceneComponent.K2_GetComponentLocation` (`self.CapsuleComponent`))))
  ;[1 1 1] GrabVine
  (`self.K2_SetActorLocation` (`KismetMathLibrary.MakeVector` _vinepos_x _vinepos_y _returnvalue_z))
  (set `self.GameMode` "NewEnumerator1")
  (set `CharacterMovementComponent.GravityScale` 0.0 _charactermovement)
  (`MovementComponent.StopMovementImmediately` _charactermovement))

(fn `EndVine`
  (set `self.CanGrab` false)
  (set `self.GameMode` "NewEnumerator0")
  (set `CharacterMovementComponent.GravityScale` 1.0 (`self.CharacterMovement`)))

(fn `SetVariable`
  (params (VineObject :type "/Game/Prefabs/Vine Object Reference") (VineTransform :type "Vector Structure"))
  (set `self.CanGrab` true)
  (set `self.Vine` VineObject)
  (set `self.VinePos` VineTransform))

(fn `UserConstructionScript`)